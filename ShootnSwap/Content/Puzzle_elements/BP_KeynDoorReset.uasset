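; A resettable key-and-door puzzle element, solved by shooting the key box with a first-person projectile.
; A projectile hit destroys the projectile and, if unsolved, teleports MovingBit to the Destination transform cached at BeginPlay and applies the toggled material.
; The Reset event, meant to be called by hazards, restores the untoggled material, moves MovingBit to ResetPoint's location and clears the Solved flag.
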(event `self.ReceiveBeginPlay`
  (set `self.Desination Transform` (`SceneComponent.K2_GetComponentToWorld` (`self.Destination`))))

(event `self.KeyBox.OnComponentHit`
  (params (HitComponent :type "PrimitiveComponent Object Reference") (OtherActor :type "Actor Object Reference") (OtherComp :type "PrimitiveComponent Object Reference") (NormalImpulse :type "Vector Structure") (Hit :type "HitResult Structure (by ref)"))
  (bind _asbp_first_person_projectile (cast `/Game/FirstPerson/Blueprints/BP_FirstPersonProjectile` OtherActor))
  (`self.K2_DestroyActor` _asbp_first_person_projectile)
  (if (not (`self.Solved`))
    (set `self.Solved` true)
    (`SceneComponent.K2_SetWorldTransform` (`self.Moving bit`) (`self.Desination Transform`) false false)
    (`PrimitiveComponent.SetMaterial` (`self.KeyBox`) 0 "/Game/Puzzle_elements/Mat_toggled.Mat_toggled")))

(event `/Game/Puzzle_elements/BPI_RecallnReset.Reset`
  (`PrimitiveComponent.SetMaterial` (`self.KeyBox`) 0 "/Game/Puzzle_elements/Mat_Untoggled.Mat_Untoggled")
  (`SceneComponent.K2_SetWorldLocationAndRotation` :`self` (`self.Moving bit`) :`NewLocation` (`SceneComponent.K2_GetComponentLocation` (`self.ResetPoint`)))
  (set `self.Solved` false))

(fn `UserConstructionScript`)