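; BP_CheckPoint is a puzzle-element checkpoint that the first-person player activates by overlapping its SetterBox and can later be recalled to.
; Activation stores the player, messages the previous checkpoint to switch off, registers itself with the player and applies an active material.
; Recall moves the player to the Arrow's location, while SetRecall clears the reference and restores the inactive material.
; PostLoadPlayerSet restores the player reference and active look after loading save data.
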(event `self.SetterBox.OnComponentBeginOverlap`
  (params (OverlappedComponent :type "PrimitiveComponent Object Reference") (OtherActor :type "Actor Object Reference") (OtherComp :type "PrimitiveComponent Object Reference") (OtherBodyIndex :type Integer) (bFromSweep :type Boolean) (SweepResult :type "HitResult Structure (by ref)"))
  (`KismetSystemLibrary.PrintString` "Player Check!")
  (bind _asbp_first_person_character (cast `/Game/FirstPerson/Blueprints/BP_FirstPersonCharacter` OtherActor))
  (`/Engine/EditorBlueprintResources/StandardMacros.IsValid` (`self.PlayerCharacter`)
    (:`Is Not Valid`
      (bind _output_get (set `self.PlayerCharacter` _asbp_first_person_character))
      (message `/Game/Puzzle_elements/BPI_RecallnReset.SetRecall` (`/Game/FirstPerson/Blueprints/BP_FirstPersonCharacter.Current_Checkpoint` _asbp_first_person_character) self) ; Call to previous checkpoint, turns it off
      (message `/Game/Puzzle_elements/BPI_RecallnReset.SetRecall` _output_get self) ; Calls to Player, sets this as the checkpoint they ask to recall to
      (`PrimitiveComponent.SetMaterial` (`self.PointBase`) 0 "/Game/Puzzle_elements/Mat_CheckActive.Mat_CheckActive" :!label _label))))

(event `/Game/Puzzle_elements/BPI_RecallnReset.Recall`
  ;[1 1 1] Respawn Logic (This event gets called on the player character)
  (`self.K2_SetActorLocation` (`self.PlayerCharacter`) (`SceneComponent.K2_GetComponentLocation` (`self.Arrow`)) false false))

(event `/Game/Puzzle_elements/BPI_RecallnReset.SetRecall`
  (params (ThisPoint :type "/Game/Puzzle_elements/BP_CheckPoint Object Reference"))
  ;[1 1 1] This event is called by other checkpoints to tell this one to deactivate
  (set `self.PlayerCharacter` null)
  (`PrimitiveComponent.SetMaterial` (`self.PointBase`) 0 "/Game/Puzzle_elements/Mat_Check.Mat_Check"))

(event `/Game/Puzzle_elements/BPI_RecallnReset.Post Load Player Set`
  (params (Player :type "/Game/FirstPerson/Blueprints/BP_FirstPersonCharacter Object Reference"))
  (set `self.PlayerCharacter` Player)
  (goto _label))

(fn `UserConstructionScript`)