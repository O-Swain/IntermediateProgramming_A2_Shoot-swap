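; BP_CourseHazard is a puzzle-course hazard that recalls an actor entering its box and resets linked puzzle elements.
; On box overlap, it checks the other actor for BPI_RecallnReset and sends it RecallMessage.
; It then sends ResetMessage to every entry in the PuzzlesReset array, printing debug text for each reset and on completion.
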(event `self.Box.OnComponentBeginOverlap`
  (params (OverlappedComponent :type "PrimitiveComponent Object Reference") (OtherActor :type "Actor Object Reference") (OtherComp :type "PrimitiveComponent Object Reference") (OtherBodyIndex :type Integer) (bFromSweep :type Boolean) (SweepResult :type "HitResult Structure (by ref)"))
  (bind _puzzlesreset (`self.PuzzlesReset`))
  (if (`KismetSystemLibrary.DoesImplementInterface` OtherActor "/Game/Puzzle_elements/BPI_RecallnReset.BPI_RecallnReset_C")
    (message `/Game/Puzzle_elements/BPI_RecallnReset.Recall` OtherActor)
    (for (_ _array_index) _puzzlesreset
      (message `/Game/Puzzle_elements/BPI_RecallnReset.Reset` (`|GetArrayItem` _puzzlesreset _array_index))
      (`KismetSystemLibrary.PrintString` (`KismetStringLibrary.Concat_StrStr` "Reset Element: " (`KismetStringLibrary.Conv_IntToString` _array_index))))
    (`KismetSystemLibrary.PrintString` "Completed Reset")))

(fn `UserConstructionScript`)