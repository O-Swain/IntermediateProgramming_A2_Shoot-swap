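; BP_CrystSpawner is a puzzle element that spawns a BP_BallCharger crystal at its Cube's location on BeginPlay and respawns it when it is gone.
; Tick checks whether the stored Crystal reference is still valid and, if not, spawns a replacement after a five-second delay.
; A DoOnce gate, reset after each spawn, prevents duplicates, and the delay is meant to stop players hovering indefinitely.
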(event `self.ReceiveBeginPlay`
  (bind _returnvalue (`|SpawnActorFromClass` "/Game/Puzzle_elements/BP_BallCharger.BP_BallCharger_C" (`KismetMathLibrary.Conv_VectorToTransform` (`SceneComponent.K2_GetComponentLocation` (`self.Cube`))) "Undefined" "MultiplyWithRoot" null null))
  (set `self.Crystal` _returnvalue))

(event `self.ReceiveTick`
  (params (DeltaSeconds :type "Float (single-precision)"))
  (`/Engine/EditorBlueprintResources/StandardMacros.IsValid` (`self.Crystal`)
    (:`Is Not Valid`
      ;[1 1 1] Puts a delay on respawn, such that player shouldn't be able to hover indefinitely
      (`/Engine/EditorBlueprintResources/StandardMacros.DoOnce` false :!label _label
        (:`Completed`
          (`KismetSystemLibrary.Delay` 5.0)
          (bind _returnvalue (`|SpawnActorFromClass` "/Game/Puzzle_elements/BP_BallCharger.BP_BallCharger_C" (`KismetMathLibrary.Conv_VectorToTransform` (`SceneComponent.K2_GetComponentLocation` (`self.Cube`))) "Undefined" "MultiplyWithRoot" null null))
          (set `self.Crystal` _returnvalue)
          (goto _label :!via `Reset`))))))

(fn `UserConstructionScript`)